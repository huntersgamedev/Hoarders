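; Enemy character Blueprint with Assault, Melee and Sniper types and a looping patrol route.
; The construction script sets the icon sprite from the enemy type and, behind a designer toggle, draws a debug sphere showing the sensing radius.
; GiveNextPatrolLocation increments the patrol index, prints a debug value, wraps to the start past the last point and returns that location.
; The event graph holds no active logic.
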(event EventBeginPlay)

(event Collision|EventActorBeginOverlap
  (params (OtherActor :type Actor%20Object%20Reference)))

(fn ConstructionScript
  (switch Utilities|FlowControl|Switch|SwitchonENU_EnemyType (Variables|Default|GetEnemyType)
    (:NewEnumerator0
      (Rendering|Components|Sprite|SetSprite (Variables|Default|GetEnemyIcon) "/Game/MyStuff/AI/AIIcons/Assaulter.Assaulter"))
    (:NewEnumerator1
      (Rendering|Components|Sprite|SetSprite (Variables|Default|GetEnemyIcon) "/Game/MyStuff/AI/AIIcons/Melee.Melee"))
    (:NewEnumerator2
      (Rendering|Components|Sprite|SetSprite (Variables|Default|GetEnemyIcon) "/Game/MyStuff/AI/AIIcons/Sniper.Sniper")))
  (if (Variables|Default|GetDESIGNER%20Show%20Senseing%20Radius)
    (Rendering|Debug|DrawDebugSphere (Transformation|GetWorldLocation (Variables|Collision|GetCapsuleComponent)) (Variables|Default|GetSensingRadius) 12 "(R=0.685218,G=0.000000,B=1.000000,A=1.000000)" 0.0)))

(fn GiveNextPatrolLocation
  (bind _result (Math|Integer|IncrementInt (Variables|Default|GetPoint%20In%20Patrol))
    (:%20%20
      (Development|PrintString (Utilities|String|ToString(Integer) _result))
      (if (> (Variables|Default|GetPoint%20In%20Patrol) (- (Utilities|Array|Length (Variables|Default|GetPatrol%20Locations)) 1))
        (Variables|Default|SetPoint%20In%20Patrol 0))
      (return (Utilities|Array|Get(acopy) (Variables|Default|GetPatrol%20Locations) (Variables|Default|GetPoint%20In%20Patrol))))))